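; BP_PickupPotionBase is a potion pickup actor, named as a base, that adds one item to the player's inventory on overlap.
; Construction disables collision, and BeginPlay re-enables it as query-only after a short delay, so the potion cannot be collected immediately on spawn.
; An overlapping LostArcPlayerCharacter receives the item through its InventoryComponent using FPickupItemName, then the actor destroys itself after a brief delay.
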(event EventBeginPlay
  (Utilities|FlowControl|Delay 3.0)
  (Collision|SetCollisionEnabled (Variables|Default|GetCollision) "QueryOnly"))

(event Collision|EventActorBeginOverlap
  (params (OtherActor :type Actor%20Object%20Reference))
  (bind _aslost_arc_player_character (Utilities|Casting|CastToLostArcPlayerCharacter OtherActor))
  (Class|LostArcInventoryComponent|AddPickupItem (Variables|/Script/LostArc.LostArcPlayerCharacter|GetInventoryComponent _aslost_arc_player_character) (Variables|Default|GetFPickupItemName) 1)
  (Utilities|FlowControl|Delay 0.1)
  (Actor|DestroyActor))

(event EventTick
  (params (DeltaSeconds :type Float%20%28single-precision%29)))

(fn ConstructionScript
  (Collision|SetCollisionEnabled (Variables|Default|GetCollision) "NoCollision"))