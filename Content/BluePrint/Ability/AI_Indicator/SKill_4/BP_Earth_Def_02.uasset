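; BP_Earth_Def_02 is a self-destroying visual effect actor for an earth defense magic skill.
; Shortly after BeginPlay it activates five earth-defense particle components and starts the TL_Earth_Def timeline.
; The timeline's De Activate All event track deactivates every particle, then the actor destroys itself after a brief delay.
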(event EventBeginPlay
  (Utilities|FlowControl|Delay 0.2)
  (Utilities|FlowControl|Sequence
    (:then_0
      ;[1 1 1] 1. Activates particle
      (Components|Activation|Activate (Variables|Default|GetPar_LMagic_Earth_Def_01a) false))
    (:then_1
      ;[1 1 1] sDeactivate_Particles
      (Timeline|TL_Earth_Def PlayFromStart
        (:DeActivate%20All
          ;[1 1 1] Deactivates Particle.
          (Components|Activation|Deactivate (Variables|Default|GetPar_LMagic_Earth_Def_01a))
          (Utilities|FlowControl|Delay 1.0)
          (Actor|DestroyActor))))))

(event Collision|EventActorBeginOverlap
  (params (OtherActor :type Actor%20Object%20Reference)))

(event EventTick
  (params (DeltaSeconds :type Float%20%28single-precision%29)))

(fn ConstructionScript)