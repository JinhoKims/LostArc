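; Timed spawner actor from the Luos8Elements content that repeatedly spawns a chosen actor class at its own transform.
; BeginPlay starts a looping timer on SpawnTime, and each tick spawns the class held in SpawnActor.
; Homing projectile classes receive Target when it is a dummy target; all other cases spawn plainly.
; The construction script forces SpawnActor to BP_Ranged_Ice_Unit, overriding any value set on the instance.
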(event Custom|Spawning
  (bind _returnvalue (Transformation|GetActorTransform))
  (bind _spawnactor (Variables|Spawning|GetSpawnActor))
  ;[1 1 1] On spawn, cast to actors.
  (bind _asbp_4e_homing_proj (Utilities|Casting|CastToBP_4E_HomingProjClass _spawnactor)
    (:then
      (bind _asbp_4e_dummy_target (Utilities|Casting|CastToBP_4E_DummyTarget (Variables|Default|GetTarget))
        (:then
          (Game|SpawnActorfromClass _asbp_4e_homing_proj _returnvalue "Undefined" 0 _asbp_4e_dummy_target 0))
        (:CastFailed
          (Game|SpawnActorfromClass _spawnactor _returnvalue "Undefined" 0 0 :!label _label))))
    (:CastFailed
      (goto _label))))

(event EventBeginPlay
  ;[1 1 1] On begin play, set timer
  (Utilities|Time|SetTimerbyEvent (delegate Custom|Spawning) (Variables|Spawning|GetSpawnTime) true))

(fn ConstructionScript
  (Variables|Spawning|SetSpawnActor "/Game/UI/Ability/RangedSkill/Ranged_1/BP_Ranged_Ice_Unit.BP_Ranged_Ice_Unit_C"))