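; BP_Circle is a self-destroying circle indicator for abilities, built from a circumference component and an area component.
; On BeginPlay it creates a dynamic material for each, using the Circum1Area0 scalar to select outline or area mode.
; After a short delay, a timeline animates the area's AreaValue parameter, then the actor destroys itself following another brief pause.
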(event EventBeginPlay
  (Utilities|FlowControl|Sequence
    (:then_0
      ;[1 1 1] Construct Material Instances
      (bind _returnvalue (Rendering|Material|CreateDynamicMaterialInstance (Variables|컴포넌트|GetCircum) :!class /Script/Engine.DecalComponent))
      (bind _output_get (Variables|Default|SetCircumRef _returnvalue))
      (Rendering|Material|SetScalarParameterValue _output_get "Circum1Area0" 1.0 :!class /Script/Engine.MaterialInstanceDynamic))
    (:then_1
      (bind _returnvalue_2 (Rendering|Material|CreateDynamicMaterialInstance (Variables|컴포넌트|GetArea) :!class /Script/Engine.DecalComponent))
      (bind _output_get_2 (Variables|Default|SetAreaRef _returnvalue_2))
      (Rendering|Material|SetScalarParameterValue _output_get_2 "Circum1Area0" 0.0 :!class /Script/Engine.MaterialInstanceDynamic))
    (:then_2
      ;[1 1 1] Play Animation
      (Utilities|FlowControl|Delay 0.1)
      (bind _areavaluealpha (Timeline|AreaValueTimeline Play)
        (:Update
          (Rendering|Material|SetScalarParameterValue (Variables|Default|GetAreaRef) "AreaValue" _areavaluealpha :!class /Script/Engine.MaterialInstanceDynamic))
        (:Finished
          (Utilities|FlowControl|Delay 0.1)
          (Actor|DestroyActor))))))

(fn ConstructionScript)