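; Wolf boss monster character that sets its combat and movement stats at construction and supplies effect events for its meteor, breath and jump-attack skills.
; Jump attack moves it to the player, switches the capsule to a falling collision profile and spawns a circular sector actor.
; Meteor spawns an actor and hands its reference to AbilityComponent.
; Breath uses a delayed-loop macro to emit a counted series of effect units from the skull socket.
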(event EventMonsterBreathEffect
  (bind _mesh (Variables|Character|GetMesh))
  ;[1 1 1] Skill_3 Breath
  (Utilities|SpawnBreath 0.1 (> 15 (Variables|Default|GetiBreathCount))
    (:Loop%20Body
      (Game|SpawnActorfromClass "/Game/BluePrint/Ability/AI_Ability/SKill_3/BP_BreathEffect_Unit.BP_BreathEffect_Unit_C" (Math|Transform|MakeTransform (Transformation|GetSocketLocation _mesh "c_skull_01_x") (Transformation|GetSocketRotation _mesh "c_skull_01_x")) "Undefined" 0 0 0)
      (Variables|Default|SetiBreathCount (+ (Variables|Default|GetiBreathCount) 1)))
    (:Exit
      (Variables|Default|SetiBreathCount 0))))

(event EventTick
  (params (DeltaSeconds :type Float%20%28single-precision%29)))

(event EventMonsterJumpEffect
  ;[1 1 1] Skill_4 JumpAttack
  (Transformation|SetActorRotation "0.000000,180.000000, 0")
  (Transformation|SetActorLocation (Transformation|GetActorLocation (Game|Player|GetPlayerPawn 0)) false false)
  (Collision|SetCollisionProfileName (Variables|Default|GetCapsuleComponent) "BossFalling" true :!class /Script/Engine.PrimitiveComponent)
  (Game|SpawnActorfromClass "/Game/BluePrint/Ability/AI_Ability/SKill_4/BP_CircularSector_Rev.BP_CircularSector_Rev_C" (Transformation|GetActorLocation) "Undefined" 0 0))

(event EventMonsterMeteorEffect
  ;[1 1 1] Skill_2 Meteor
  (bind _returnvalue (Game|SpawnActorfromClass "/Game/BluePrint/Ability/AI_Ability/SKill_2/BP_Meteor.BP_Meteor_C" (Math|Conversions|ToTransform(Vector) (Transformation|GetActorLocation)) "Undefined" 0 0))
  (Variables|/Script/LostArc.AIAbilityComponent|SetMeteorActorRef (Variables|Default|GetAbilityComponent) _returnvalue))

(fn ConstructionScript
  (Variables|Default|SetBasicAttackRange 3e+02)
  (Variables|Default|SetMonsterHP 1e+02)
  (Variables|Default|SetMonsterRotateSpeed 128.0)
  (bind _output_get (Variables|Default|SetMonsterSpeed 4e+02))
  (Variables|/Script/Engine.CharacterMovementComponent|SetMaxWalkSpeed (Variables|Character|GetCharacterMovement) _output_get))

(fn MonsterBreath
  (bind _mesh (Variables|Character|GetMesh))
  (Game|SpawnActorfromClass "/Game/BluePrint/Ability/AI_Ability/SKill_3/BP_BreathEffect_Unit.BP_BreathEffect_Unit_C" (Math|Transform|MakeTransform (Transformation|GetSocketLocation _mesh "c_skull_01_x") (Transformation|GetSocketRotation _mesh "c_skull_01_x")) "Undefined" 0 0 0))