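; Aiming indicator actor for the player's fourth ranged skill, with a cone sprite that points toward the mouse.
; Each tick it follows the player character at a lowered height and rotates using a look-at between its projected screen position and the cursor, computed in screen space.
; On BeginPlay it binds to the RangedEffectCheck delegate of the RangedSpell4 ability (LostArcSkill_8) and destroys itself when that fires.
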(event Custom|be%20activated%20Spawn%20Effects
  (params (Type :type EAbilityType%20Enum :default "BasicAttack"))
  ;[1 1 1] Delegate Binding
  (Actor|DestroyActor))

(event EventBeginPlay
  ;[1 1 1] Delegate Binding
  (bind _aslost_arc_player_character (Utilities|Casting|CastToLostArcPlayerCharacter (Game|GetPlayerCharacter 0)))
  (bind _returnvalue (Class|LostArcCharacterAbilityComponent|GetAbilities (Variables|/Script/LostArc.LostArcPlayerCharacter|GetAbilityComponent _aslost_arc_player_character) "RangedSpell_4"))
  (bind _aslost_arc_skill_8 (Utilities|Casting|CastToLostArcSkill_8 _returnvalue))
  (EventDispatchers|AssignOnRangedEffectCheck _aslost_arc_skill_8 (delegate Custom|be%20activated%20Spawn%20Effects)))

(event Collision|EventActorBeginOverlap
  (params (OtherActor :type Actor%20Object%20Reference)))

(event EventTick
  (params (DeltaSeconds :type Float%20%28single-precision%29))
  (bind _returnvalue (Game|GetPlayerController 0))
  (bind _returnvalue_2 (Game|GetPlayerController 0))
  (bind _returnvalue_3 (Game|GetPlayerCharacter 0))
  (bind _returnvalue_4 (Transformation|GetActorLocation))
  (bind _z (Math|Vector|BreakVector _returnvalue_4))
  (bind (_locationx _locationy) (Game|Player|GetMousePosition _returnvalue_2))
  (bind _returnvalue_5 (Transformation|GetActorLocation _returnvalue_3))
  (bind _screenlocation (Class|PlayerController|ProjectWorldLocationtoScreen _returnvalue _returnvalue_4 false))
  (bind (_x _y) (Math|Vector2D|BreakVector2D _screenlocation))
  (bind (_x_2 _y_2 _z_2) (Math|Vector|BreakVector _returnvalue_5))
  ;[1 1 1] Indicator Tracking Mouse
  (Transformation|SetActorRotation (Math|Rotator|FindLookatRotation (Math|Vector|MakeVector _x _y _z) (Math|Vector|MakeVector _locationx _locationy _z)))
  (Transformation|SetActorLocation (Math|Vector|MakeVector _x_2 _y_2 (- _z_2 1e+02)) false false))

(fn ConstructionScript
  (Collision|SetCollisionObjectType (Variables|Default|GetconeSkill_Sprite_1) "ECC_Visibility"))