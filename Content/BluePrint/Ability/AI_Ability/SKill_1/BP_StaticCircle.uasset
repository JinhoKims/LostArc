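; Short-lived circle effect actor for an AI ability (Skill 1) that spins in a randomly chosen direction.
; On BeginPlay it creates a dynamic material for Circle and sets its angle parameter, leaving CircleRvs's material untouched.
; A random bool reveals either Circle or CircleRvs and plays the matching timeline to drive the CircleRoot's yaw.
; The actor destroys itself shortly after the timeline finishes.
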(event EventBeginPlay
  (Utilities|FlowControl|Sequence
    (:then_0
      ;[1 1 1] Construct Material Instances
      (bind _returnvalue (Rendering|Material|CreateDynamicMaterialInstance (Variables|컴포넌트|GetCircle) :!class /Script/Engine.DecalComponent))
      (bind _output_get (Variables|Default|SetCircleRef _returnvalue))
      (Rendering|Material|SetScalarParameterValue _output_get "AngleParm" 9e+01 :!class /Script/Engine.MaterialInstanceDynamic))
    (:then_1
      (if (Math|Random|RandomBool)
        ;[1 1 1] Rotate to Circle L
        (Rendering|SetVisibility (Variables|컴포넌트|GetCircle) true false)
        (bind _newtrack (Timeline|RoatateTickScale Play)
          (:Update
            (Transformation|SetRelativeRotation (Variables|Default|GetCircleRoot) (Math|Rotator|MakeRotator 0.0 0.0 _newtrack) false false))
          (:Finished
            (Utilities|FlowControl|Delay 0.2)
            (Actor|DestroyActor)))
        (else
          ;[1 1 1] Rotate to Circle L
          (Rendering|SetVisibility (Variables|Default|GetCircleRvs) true false)
          (bind _rvstrack (Timeline|RotateTickScale_Rvs Play)
            (:Update
              (Transformation|SetRelativeRotation (Variables|Default|GetCircleRoot) (Math|Rotator|MakeRotator 0.0 0.0 _rvstrack) false false))
            (:Finished
              (Utilities|FlowControl|Delay 0.2)
              (Actor|DestroyActor))))))))

(fn ConstructionScript)