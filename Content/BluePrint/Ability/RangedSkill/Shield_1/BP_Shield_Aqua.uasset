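; BP_Shield_Aqua is the water shield skill effect that surrounds player character 0 and then removes itself.
; On BeginPlay it activates its aqua defense particle and scales it from zero to full with one timeline, then a second timeline shrinks it back.
; The shrink's Update starts a one-second Delay before destroying the actor.
; Tick snaps the actor to the player's location every frame, without attachment.
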(event EventTick
  (params (DeltaSeconds :type Float%20%28single-precision%29))
  (Transformation|SetActorLocation (.Location (Math|Transform|BreakTransform (Transformation|GetActorTransform (Game|GetPlayerCharacter 0)))) false false))

(event EventBeginPlay
  (bind _par_lmagic_aqua_def_01 (Variables|Default|GetPar_LMagic_Aqua_Def_01))
  (Components|Activation|Activate _par_lmagic_aqua_def_01 false)
  (bind _aqua_def_time (Timeline|TL_Aqua_On PlayFromStart)
    (:Update
      (Transformation|SetRelativeScale3D _par_lmagic_aqua_def_01 (Math|Vector|Lerp(Vector) "0, 0, 0" "1.000000,1.000000,1.000000" _aqua_def_time)))
    (:Finished
      (bind _aqua_def_time_2 (Timeline|TL_Aqua_Off Play)
        (:Update
          (Transformation|SetRelativeScale3D _par_lmagic_aqua_def_01 (Math|Vector|Lerp(Vector) "1.000000,1.000000,1.000000" "0, 0, 0" _aqua_def_time_2))
          (Utilities|FlowControl|Delay 1.0)
          (Actor|DestroyActor))))))

(fn ConstructionScript)