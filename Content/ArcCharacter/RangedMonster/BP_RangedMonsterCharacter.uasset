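; BP_RangedMonsterCharacter is a ranged monster character that can drop a pickup item.
; The construction script sets its attack range, HP, rotation and movement speeds, and applies the movement speed to CharacterMovement's MaxWalkSpeed.
; The DropPickupItem event spawns one of the first two SpawnType classes at random at the monster's transform.
; BeginPlay, overlap and Tick events are empty.
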(event EventBeginPlay)

(event Collision|EventActorBeginOverlap
  (params (OtherActor :type Actor%20Object%20Reference)))

(event EventTick
  (params (DeltaSeconds :type Float%20%28single-precision%29)))

(event EventDropPickupItem
  (Game|SpawnActorfromClass (Utilities|Array|Get(acopy) (Variables|Default|GetSpawnType) (Math|Random|RandomIntegerinRange 0 1)) (Transformation|GetActorTransform) "Undefined" 0 0))

(fn ConstructionScript
  (Variables|Default|SetBasicAttackRange 6e+02)
  (Variables|Default|SetMonsterHP 1e+02)
  (Variables|Default|SetMonsterRotateSpeed 64.0)
  (bind _output_get (Variables|Default|SetMonsterSpeed 2e+02))
  (Variables|/Script/Engine.CharacterMovementComponent|SetMaxWalkSpeed (Variables|Character|GetCharacterMovement) _output_get))